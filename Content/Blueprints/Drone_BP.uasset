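; Player-controlled drone Blueprint that flies by physics on its Collision component.
; Mouse and pitch/roll axes add torque, while Tick damps spin, applies downward force and blends velocity toward forward times throttle.
; Q/E set flags for the Throttle function, but its looping timer setup is unconnected, as is a drone-spawning node.
; BeginPlay switches the view to MiniCam; C and Z set camera FOVs to zero.
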(event `InputAxisKey|MouseY`
  (params (AxisValue :type "Float (single-precision)"))
  (bind _returnvalue (* AxisValue -200.0))
  (set `self.MouseY` AxisValue)
  (`PrimitiveComponent.AddTorqueInDegrees` (`self.collision`) (`KismetMathLibrary.VLerp` (0.0 0.0 0.0) (* (`SceneComponent.GetRightVector` (`self.collision`)) (`KismetMathLibrary.SelectFloat` _returnvalue (/ _returnvalue 1.0) (> (`self.CurrentThrottle`) 0.0))) 0.1) "None" true))

(event `InputAxis|roll`
  (params (AxisValue :type "Float (single-precision)"))
  (bind _returnvalue (* AxisValue -200.0))
  (set `self.MouseX` AxisValue)
  (`PrimitiveComponent.AddTorqueInDegrees` (`self.collision`) (`KismetMathLibrary.VLerp` (0.0 0.0 0.0) (* (`SceneComponent.GetForwardVector` (`self.collision`)) (`KismetMathLibrary.SelectFloat` _returnvalue (/ _returnvalue 1.0) (> (`self.CurrentThrottle`) 0.0))) 0.1) "None" true))

(event `InputAxisKey|MouseX`
  (params (AxisValue :type "Float (single-precision)"))
  (bind _returnvalue (* AxisValue -200.0))
  (set `self.MouseX` AxisValue)
  (`PrimitiveComponent.AddTorqueInDegrees` (`self.collision`) (`KismetMathLibrary.VLerp` (0.0 0.0 0.0) (* (`SceneComponent.GetForwardVector` (`self.collision`)) (`KismetMathLibrary.SelectFloat` _returnvalue (/ _returnvalue 1.0) (> (`self.CurrentThrottle`) 0.0))) 0.1) "None" true))

(event `InputAxis|pitch`
  (params (AxisValue :type "Float (single-precision)"))
  (bind _returnvalue (* AxisValue -200.0))
  (set `self.MouseY` AxisValue)
  (`PrimitiveComponent.AddTorqueInDegrees` (`self.collision`) (`KismetMathLibrary.VLerp` (0.0 0.0 0.0) (* (`SceneComponent.GetRightVector` (`self.collision`)) (`KismetMathLibrary.SelectFloat` _returnvalue (/ _returnvalue 1.0) (> (`self.CurrentThrottle`) 0.0))) 0.1) "None" true))

(event `Key|Q`
  (params (Key :type "Key Structure"))
  (:`Pressed`
    (set `self.MoveThrottleUp` true))
  (:`Released`
    (set `self.MoveThrottleUp` false)))

(event `Key|E`
  (params (Key :type "Key Structure"))
  (:`Pressed`
    (set `self.MoveThrottleDown` false))
  (:`Released`
    (set `self.MoveThrottleDown` true)))

(event `self.ReceiveTick`
  (params (DeltaSeconds :type "Float (single-precision)"))
  (bind _collision (`self.collision`))
  (`|ExecutionSequence`
    (:`then_0`
      (`PrimitiveComponent.AddTorqueInDegrees` _collision (/ (`KismetMathLibrary.NegateVector` (`PrimitiveComponent.GetPhysicsAngularVelocityInDegrees` (`self.collision`) "None")) 0.75) "None" false)
      (`PrimitiveComponent.AddForce` _collision (0.0 0.0 -1500.0) "None" true)
      (`self.Speed`))
    (:`then_1`
      (if (`self.ZeroThrottle`)
        (set `self.CurrentThrottle` (`KismetMathLibrary.FInterpTo_Constant` (`self.CurrentThrottle`) 0.0 (`GameplayStatics.GetWorldDeltaSeconds`) 500.0))))))

(event `Key|C`
  (params (Key :type "Key Structure"))
  (:`Pressed`
    (`CameraComponent.SetFieldOfView` (`self.miniCamera`) 0.0)))

(event `Key|Z`
  (params (Key :type "Key Structure"))
  (:`Pressed`
    (`CameraComponent.SetFieldOfView` (`self.Camera1`) 0.0)))

(event `self.ReceiveBeginPlay`
  (`PlayerController.SetViewTargetWithBlend` (`GameplayStatics.GetPlayerController` 0) (`self.MiniCam`) 0.0 "VTBlend_Linear" 0.0 false))

(event `OnComponentBeginOverlap_Event`
  (params (OverlappedComponent :type "PrimitiveComponent Object Reference") (OtherActor :type "Actor Object Reference") (OtherComp :type "PrimitiveComponent Object Reference") (OtherBodyIndex :type Integer) (bFromSweep :type Boolean) (SweepResult :type "HitResult Structure (by ref)")))

(fn `Speed`
  (locals (NewLocalVar_0 :type "Vector Structure" :default (0.0 0.0 0.0)))
  (bind _returnvalue (`PrimitiveComponent.GetPhysicsLinearVelocity` (`self.collision`) "None"))
  (`PrimitiveComponent.SetPhysicsLinearVelocity` (`self.collision`) (`KismetMathLibrary.VLerp` _returnvalue (* (`SceneComponent.GetForwardVector` (`self.collision`)) (* (`self.CurrentThrottle`) 500.0)) 0.1) false "None"))

(fn `Throttle`
  (`|ExecutionSequence`
    (:`then_0`
      (if (`self.MoveThrottleUp`)
        (set `self.CurrentThrottle` (`KismetMathLibrary.FClamp` (+ (`self.CurrentThrottle`) 1.0) 0.0 750.0))
        (elif (`self.MoveThrottleDown`)
          (set `self.CurrentThrottle` (`KismetMathLibrary.FClamp` (+ (`self.CurrentThrottle`) -1.0) 0.0 750.0)))))))

(fn `UserConstructionScript`)